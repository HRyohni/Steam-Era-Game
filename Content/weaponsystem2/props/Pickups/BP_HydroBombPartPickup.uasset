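; BP_HydroBombPartPickup is an interactable pickup for a hydro bomb part that also advances the story.
; On Interact, it casts player pawn 0 to BP_FirstPersonCharacter, increments that character's HydroBombParts count and prints the new total.
; It then destroys itself and increments the character's StoryLine counter.
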(event EventBeginPlay
  (|CallParentFunction) ; This node is disabled and will not be called.\nDrag off pins to build functionality.
)

(event Collision|EventActorBeginOverlap
  (params (OtherActor :type Actor%20Object%20Reference))
  (|CallParentFunction OtherActor) ; This node is disabled and will not be called.\nDrag off pins to build functionality.
)

(event EventTick
  (params (DeltaSeconds :type Float%20%28single-precision%29))
  (|CallParentFunction DeltaSeconds) ; This node is disabled and will not be called.\nDrag off pins to build functionality.
)

(event EventInteract
  (params (Character%20Picking%20up :type BP%20First%20Person%20Character%20Object%20Reference))
  (bind _asbp_first_person_character (Utilities|Casting|CastToBP_FirstPersonCharacter (Game|Player|GetPlayerPawn 0)))
  (bind _output_get (Variables|/Game/FirstPerson/Blueprints/BP_FirstPersonCharacter.BP_FirstPersonCharacter_C|SetHydroBombParts _asbp_first_person_character (+ 1 (Variables|/Game/FirstPerson/Blueprints/BP_FirstPersonCharacter.BP_FirstPersonCharacter_C|GetHydroBombParts _asbp_first_person_character))))
  (Development|PrintString (Utilities|String|ToString(Integer) _output_get))
  (Actor|DestroyActor)
  (bind _result (Math|Integer|IncrementInt (Variables|/Game/FirstPerson/Blueprints/BP_FirstPersonCharacter.BP_FirstPersonCharacter_C|GetstoryLine _asbp_first_person_character))
    (:%20%20
      (Variables|/Game/FirstPerson/Blueprints/BP_FirstPersonCharacter.BP_FirstPersonCharacter_C|SetstoryLine _asbp_first_person_character _result))))

(fn ConstructionScript
  (|CallParentFunction))