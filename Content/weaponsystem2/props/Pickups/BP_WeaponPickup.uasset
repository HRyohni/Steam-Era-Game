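; BP_WeaponPickup is a weapon pickup that gives a weapon to the character that interacts with it.
; Its Interact event calls SpawnWeapon on that character, passing its WeaponToSpawn and its own location, then destroys itself and plays a 2D pistol ammo pickup sound.
; Pickup runs only through Interact, as the overlap and tick events are disabled and the construction script only calls its parent.
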(event EventBeginPlay
  (|CallParentFunction) ; This node is disabled and will not be called.\nDrag off pins to build functionality.
)

(event Collision|EventActorBeginOverlap
  (params (OtherActor :type Actor%20Object%20Reference))
  (|CallParentFunction OtherActor) ; This node is disabled and will not be called.\nDrag off pins to build functionality.
)

(event EventTick
  (params (DeltaSeconds :type Float%20%28single-precision%29))
  (|CallParentFunction DeltaSeconds) ; This node is disabled and will not be called.\nDrag off pins to build functionality.
)

(event EventInteract
  (params (Character%20Picking%20up :type BP%20First%20Person%20Character%20Object%20Reference))
  (Default|SpawnWeapon Character%20Picking%20up (Variables|Default|GetWeaponToSpawn) (Transformation|GetActorLocation))
  (Actor|DestroyActor)
  (Audio|PlaySound2D "/Game/MilitaryWeapSilver/Sound/Pistol/Cues/Pistol_AmmoPickup_Cue.Pistol_AmmoPickup_Cue" 1.0 1.0 0.0 0 0))

(fn ConstructionScript
  (|CallParentFunction))