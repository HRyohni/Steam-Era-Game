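; BP_DefaultDialogue is a default NPC dialogue actor that steps through an array of lines, one per Talk call.
; Each step shows the line and speaker name (fallback "Robot") in WB_Dialogue, blends the view to the NPC camera and plays a voice sound once.
; After the last line it removes the widget and blends back to the player.
; Talk hides the player without unhiding it here; trigger overlap events are empty.
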(event OnComponentBeginOverlap(TriggerZone)
  (params (OverlappedComponent :type Primitive%20Component%20Object%20Reference) (OtherActor :type Actor%20Object%20Reference) (OtherComp :type Primitive%20Component%20Object%20Reference) (OtherBodyIndex :type Integer) (bFromSweep :type Boolean) (SweepResult :type Hit%20Result%20Structure%20%28by%20ref%29))
  ;[1 1 1] talk widget
)

(event OnComponentEndOverlap(TriggerZone)
  (params (OverlappedComponent :type Primitive%20Component%20Object%20Reference) (OtherActor :type Actor%20Object%20Reference) (OtherComp :type Primitive%20Component%20Object%20Reference) (OtherBodyIndex :type Integer))
  ;[1 1 1] talk widget
)

(event Custom|DefaultFunction
  (bind _widget (Variables|Default|GetWidget))
  (bind _caractername (Variables|Default|GetCaracterName))
  (bind _returnvalue (Utilities|Text|ToText(String) _caractername))
  (Utilities|IsValid _widget
    (:Is%20Valid
      (Components|DestroyComponent _widget))
    (:Is%20Not%20Valid
      _))
  (Math|Integer|IncrementInt (Variables|Default|GettalkIndex)
    (:%20%20
      (if (< (Variables|Default|GettalkIndex) (Utilities|Array|Length (Variables|Default|GetDialogue)))
        (Variables|Default|GetNewVar
          (:then
            _)
          (:else
            (bind _returnvalue_2 (UserInterface|CreateWidget "/Game/NPC/Dialogue/WB_Dialogue.WB_Dialogue_C" (Game|GetPlayerController 0)))
            (bind _output_get (Variables|Default|SetNewVar _returnvalue_2))
            (UserInterface|Viewport|AddtoViewport _output_get 0)))
        (Rendering|Components|TextRender|SetText (Variables|/Game/NPC/Dialogue/WB_Dialogue.WB_Dialogue_C|GetTalkText (Variables|Default|GetNewVar)) (Utilities|Text|ToText(String) (Utilities|Array|Get(acopy) (Variables|Default|GetDialogue) (Variables|Default|GettalkIndex))))
        (if (Utilities|Text|TextIsEmpty _returnvalue)
          (Rendering|Components|TextRender|SetText (Variables|/Game/NPC/Dialogue/WB_Dialogue.WB_Dialogue_C|GetcaracterName (Variables|Default|GetNewVar)) "Robot")
          (else
            (Rendering|Components|TextRender|SetText (Variables|/Game/NPC/Dialogue/WB_Dialogue.WB_Dialogue_C|GetcaracterName (Variables|Default|GetNewVar)) _returnvalue)))
        (bind _asbp_first_person_character (Utilities|Casting|CastToBP_FirstPersonCharacter (Game|GetPlayerCharacter 0)))
        (if (Utilities|IsValid _asbp_first_person_character)
          (bind _asplayer_controller (Utilities|Casting|CastToPlayerController (Pawn|GetController _asbp_first_person_character)))
          (if (Utilities|IsValid _asplayer_controller)
            (Game|Player|SetViewTargetwithBlend _asplayer_controller (Components|GetOwner (Variables|Default|GetCamera)) 0.5 "VTBlend_Linear" 0.0 false)
            (Utilities|FlowControl|DoOnce false
              (:Completed
                (bind _returnvalue_3 (Audio|SpawnSound2D "/Game/NPC/Dialogue/sound/talk1.talk1" 1.0 1.0 0.0 0))
                (Components|Activation|SetActive _returnvalue_3 true false)))))
        (else
          (Widget|RemovefromParent (Variables|Default|GetNewVar))
          (bind _asbp_first_person_character_2 (Utilities|Casting|CastToBP_FirstPersonCharacter (Game|GetPlayerCharacter 0)))
          (if (Utilities|IsValid _asbp_first_person_character_2)
            (bind _asplayer_controller_2 (Utilities|Casting|CastToPlayerController (Pawn|GetController _asbp_first_person_character_2)))
            (if (Utilities|IsValid _asplayer_controller_2)
              (bind _returnvalue_4 (Actor|GetActorOfClass "/Game/FirstPerson/Blueprints/BP_FirstPersonCharacter.BP_FirstPersonCharacter_C"))
              (Game|Player|SetViewTargetwithBlend _asplayer_controller_2 _returnvalue_4 0.5 "VTBlend_Linear" 0.0 false))))))))

(event EventTalk
  (bind _asbp_first_person_character (Utilities|Casting|CastToBP_FirstPersonCharacter (Game|Player|GetPlayerPawn 0)))
  (Rendering|SetActorHiddenInGame _asbp_first_person_character true)
  (CallFunction|DefaultFunction)
  (Rendering|SetActorHiddenInGame _asbp_first_person_character true))

(fn ConstructionScript)