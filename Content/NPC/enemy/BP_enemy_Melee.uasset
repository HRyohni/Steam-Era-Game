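; Melee enemy Blueprint that supplies sword attack, equip and unequip behavior on top of a parent class.
; Montage notifies time the gameplay: spawning the sword onto the hand socket, destroying it, and firing a forward sphere trace that damages the pawn it hits.
; The attack makes the damage component non-interruptible until the montage completes or is interrupted, then signals attack end.
; Equip and unequip dispatch their events when their montages complete.
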(event EventBeginPlay
  (|CallParentFunction))

(event EventUnequipWeapon
  (bind _notifyname (Animation|Montage|PlayMontage (Variables|Character|GetMesh) "/Game/NPC/Montage_Sheath_sword.Montage_Sheath_sword")
    (:OnCompleted
      (Default|CallOnWeaponUnequipped))
    (:OnNotifyBegin
      (switch name _notifyname
        (:DropSword
          (Actor|DestroyActor (Variables|Default|GetWeaponActor))
          (Variables|Default|SetIsWieldingWeapon false))))))

(event Collision|EventActorBeginOverlap
  (params (OtherActor :type Actor%20Object%20Reference)))

(event EventTick
  (params (DeltaSeconds :type Float%20%28single-precision%29)))

(event EventAttack
  (bind _returnvalue (Transformation|GetActorLocation))
  (bind _notifyname (Animation|Montage|PlayMontage (Variables|Character|GetMesh) "/Game/NPC/Montage_swordslash.Montage_swordslash")
    (:then
      (Variables|/Game/NPC/DamageSystem/BPC_DamageSystem.BPC_DamageSystem_C|SetIsInterruptable (Variables|Default|GetBPC_DamageSystem) false))
    (:OnCompleted
      (Default|CallOnAttackEnd :!label _label)
      (Variables|/Game/NPC/DamageSystem/BPC_DamageSystem.BPC_DamageSystem_C|SetIsInterruptable (Variables|Default|GetBPC_DamageSystem) true))
    (:OnInterrupted
      (goto _label))
    (:OnNotifyBegin
      (switch name _notifyname
        (:Slash
          (bind (_outhit _returnvalue_2) (Collision|SphereTraceForObjects _returnvalue (+ _returnvalue (* (Transformation|GetActorForwardVector) 2e+02)) 2e+01 (Utilities|Array|MakeArray "ObjectTypeQuery3") false 0 "ForDuration"))
          (if _returnvalue_2
            (Class|BPIDamagable|TakeDamage(Message) (.HitActor (Collision|BreakHitResult _outhit)) (Utilities|Struct|MakeS_DamageInfo 25.0 "NewEnumerator1"))))))))

(event EventEquipWeapon
  (bind _notifyname (Animation|Montage|PlayMontage (Variables|Character|GetMesh) "/Game/NPC/Montage_Unsheath_sword.Montage_Unsheath_sword")
    (:OnCompleted
      (Default|CallOnWeaponEquipped))
    (:OnNotifyBegin
      (switch name _notifyname
        (:HoldSword
          (bind _returnvalue (Game|SpawnActorfromClass "/Game/NPC/Weapons/BP_Weapon_Sword.BP_Weapon_Sword_C" (Transformation|GetActorTransform) "Undefined" "MultiplyWithRoot" 0 0))
          (bind _output_get (Variables|Default|SetWeaponActor _returnvalue))
          (Transformation|AttachComponentToComponent _output_get (Variables|Character|GetMesh) "hand_r_sword_socket" "SnapToTarget" "SnapToTarget" "SnapToTarget" true)
          (Variables|Default|SetIsWieldingWeapon true))))))

(fn ConstructionScript
  (|CallParentFunction))