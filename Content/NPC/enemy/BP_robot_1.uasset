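; Robot enemy NPC that spawns a rifle on a mesh socket and fights the target chosen by its AI controller.
; Attack plays a firing montage whose notify damages the target when a visibility trace is unobstructed.
; Incoming damage feeds the damage component; death triggers an explosion, destroys robot and rifle, and randomly drops a coin suitcase or canister.
; It also supplies movement speeds, ideal combat ranges and hardcoded health values.
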(event Game|Damage|EventAnyDamage
  (params (Damage :type Float%20%28single-precision%29) (DamageType :type Damage%20Type%20Object%20Reference) (InstigatedBy :type Controller%20Object%20Reference) (DamageCauser :type Actor%20Object%20Reference))
  (bind _returnvalue (Transformation|GetActorLocation))
  (bind _returnvalue_2 (Math|Conversions|ToTransform(Vector) _returnvalue))
  (Default|TakeDamage (Variables|Default|GetBPC_DamageSystem) (Utilities|Struct|MakeS_DamageInfo Damage "NewEnumerator2" "NewEnumerator1"))
  (bind _dead (CallFunction|IsDead))
  (if _dead
    (Effects|SpawnEmitteratLocation "/Game/StarterContent/Particles/P_Explosion.P_Explosion" _returnvalue "0, 0, 0" "5.000000,5.000000,5.000000")
    (Audio|SpawnSoundatLocation "/Game/StarterContent/Audio/Explosion01.Explosion01" _returnvalue "0, 0, 0" 1.0 1.0 0.0 0 0)
    (Actor|DestroyActor)
    (Actor|DestroyActor (stale EventEquipWeapon _returnvalue))
    (if (Math|Random|RandomBool)
      (Game|SpawnActorfromClass "/Game/UI/suitCaseOfCoins-10/suitCaseOfCoins.suitCaseOfCoins_C" _returnvalue_2 "Undefined" "MultiplyWithRoot" 0 0)
      (else
        (Game|SpawnActorfromClass "/Game/UI/canister-health35/canister.canister_C" _returnvalue_2 "Undefined" "MultiplyWithRoot" 0 0)))))

(event EventBeginPlay
  (CallFunction|EquipWeapon))

(event EventEquipWeapon
  (bind _returnvalue (Game|SpawnActorfromClass "/Game/NPC/Weapons/BP_Weapon_Rifle.BP_Weapon_Rifle_C" (Math|Transform|MakeTransform "0, 0, 0") "Undefined" "MultiplyWithRoot" 0 0))
  (bind _output_get (Variables|Default|SetWeaponActor _returnvalue))
  (Transformation|AttachComponentToComponent _output_get (Variables|Character|GetMesh) "rifle_socket_robot" "SnapToTarget" "SnapToTarget" "SnapToTarget" true)
  (Variables|Default|SetIsWieldingWeapon true)
  (Default|CallOnWeaponEquipped))

(event EventAttack
  (bind _notifyname (Animation|Montage|PlayMontage (Variables|Character|GetMesh) "/Game/NPC/enemy/Animacije/Robot_one/Montage_one_firing_rifle.Montage_one_firing_rifle")
    (:OnCompleted
      (Default|CallOnAttackEnd :!label _label))
    (:OnInterrupted
      (goto _label))
    (:OnNotifyBegin
      (switch name _notifyname
        (:Fire
          (bind _asaic_enemy_base (Utilities|Casting|CastToAIC_enemy_base (AI|GetAIController self)))
          (bind _attack_target (Variables|/Game/NPC/enemy/AI/AIC_enemy_base.AIC_enemy_base_C|GetAttack%20Target _asaic_enemy_base)
            (:then
              (bind _returnvalue (Collision|LineTraceByChannel (Transformation|GetActorLocation (Variables|Default|GetWeaponActor)) (Transformation|GetActorLocation _attack_target) "TraceTypeQuery1" false 0 "ForDuration"))
              (if (not _returnvalue)
                (Class|BPIDamagable|TakeDamage(Message) _attack_target (Utilities|Struct|MakeS_DamageInfo 2e+01 "NewEnumerator0"))))
            (:else)))))))

(fn ConstructionScript
  (|CallParentFunction))

(fn SetMovementSpeed
  (params (Speed :type E_MovementSpeed%20Enum :default "NewEnumerator0"))
  (Variables|/Script/Engine.CharacterMovementComponent|SetMaxWalkSpeed (Variables|Character|GetCharacterMovement) (Utilities|Select :Index Speed :NewEnumerator0 0.0 :NewEnumerator1 2e+02 :NewEnumerator2 3e+02 :NewEnumerator3 5e+02))
  (return 0.0))

(fn GetIdealRange
  (return 6e+02 6e+02))

(fn TakeDamage
  (params (DamageInfo :type S%20Damage%20Info%20Structure))
  (bind _wasdamaged (Default|TakeDamage (Variables|Default|GetBPC_DamageSystem) DamageInfo))
  (return _wasdamaged))

(fn GetCurrentHealth
  (return 1e+02))

(fn GetMaxHealth
  (return 1e+02))