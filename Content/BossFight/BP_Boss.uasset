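; Boss character for a boss fight, with its own on-screen health bar, a traced attack and an explosive death.
; The Attack event plays a montage whose notify fires a forward line trace for damage and sound, plus a world camera shake.
; AnyDamage lowers Health, which Tick pushes to the widget.
; At zero health it stops movement, ragdolls and, once, spawns explosion effects, disables capsule collision and blocks further attacks.
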(event EventBeginPlay
  (bind _returnvalue (UserInterface|CreateWidget "/Game/BossFight/WB_BossHealth.WB_BossHealth_C"))
  (UserInterface|Viewport|AddtoViewport _returnvalue 0)
  (Variables|Default|SetHealthBarUi _returnvalue))

(event EventAttack
  (bind _attackpos (Variables|Default|GetAttackPos))
  (bind _returnvalue (Transformation|GetWorldLocation _attackpos))
  ;[1 1 1] attack
  (if (and (not (Variables|Default|GetisAttacking?)) (not (Variables|Default|GetisDead)))
    (Animation|Montage|PlayMontage (Variables|Character|GetMesh) "/Game/Ancient_Golem/Demo/ThirdPersonJump_Start_Montage.ThirdPersonJump_Start_Montage"
      (:then
        (Variables|Default|SetisAttacking? true))
      (:OnCompleted
        (Variables|Default|SetisAttacking? false))
      (:OnNotifyBegin
        (Utilities|FlowControl|Sequence
          (:then_0
            (bind (_outhit _returnvalue_2) (Collision|LineTraceByChannel _returnvalue (+ _returnvalue (* (Math|Vector|GetForwardVector (Transformation|GetWorldRotation _attackpos)) 1.5e+03)) "TraceTypeQuery1" false 0 "ForDuration"))
            (if _returnvalue_2
              (Game|Damage|ApplyDamage (.HitActor (Collision|BreakHitResult _outhit)) 2e+01 0 0)
              (Audio|PlaySound2D "/Game/MilitaryWeapSilver/Sound/Knife/Wavs/KnifeA_Swing01.KnifeA_Swing01" 1.0 1.0 0.0 0 0)))
          (:then_1
            (Camera|PlayWorldCameraShake "/Game/BossFight/BP_AttackCameraShake.BP_AttackCameraShake_C" (Transformation|GetActorLocation) 0.0 3.5e+03)))))))

(event EventTick
  (params (DeltaSeconds :type Float%20%28single-precision%29))
  (Progress|SetPercent (Variables|/Game/BossFight/WB_BossHealth.WB_BossHealth_C|GetHealthBar (Variables|Default|GetHealthBarUi)) (/ (Variables|Default|Gethealth) 1e+02)))

(event Game|Damage|EventAnyDamage
  (params (Damage :type Float%20%28single-precision%29) (DamageType :type Damage%20Type%20Object%20Reference) (InstigatedBy :type Controller%20Object%20Reference) (DamageCauser :type Actor%20Object%20Reference))
  (bind _mesh (Variables|Character|GetMesh))
  (bind _returnvalue (Transformation|GetWorldLocation _mesh))
  (Variables|Default|Sethealth (- (Variables|Default|Gethealth) Damage))
  (if (<= (Variables|Default|Gethealth) 0.0)
    (Pawn|Components|CharacterMovement|DisableMovement (Variables|Character|GetCharacterMovement))
    (Physics|SetSimulatePhysics (Variables|Character|GetMesh) true)
    (Utilities|FlowControl|DoOnce false
      (:Completed
        (Effects|SpawnEmitteratLocation "/Game/StarterContent/Particles/P_Explosion.P_Explosion" _returnvalue "0, 0, 0" "11.000000,11.000000,11.000000")
        (Effects|SpawnEmitteratLocation "/Game/StarterContent/Particles/P_Fire.P_Fire" _returnvalue "0, 0, 0" "5.000000,5.000000,5.000000")
        (Audio|PlaySoundatLocation "/Game/StarterContent/Audio/Explosion01.Explosion01" (Transformation|GetWorldLocation (Variables|Character|GetMesh)) "0, 0, 0" 1.0 1.0 0.0 0 0 0 0)
        (Variables|Default|SetisDead true)
        (Collision|SetCollisionEnabled (Variables|Collision|GetCapsuleComponent) "NoCollision")))))

(fn ConstructionScript)